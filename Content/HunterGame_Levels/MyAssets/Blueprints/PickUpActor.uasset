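; PickUpActor is a time bonus pickup that adds seconds to the remaining time on the player's HUD.
; The first overlap of its Box, with no check on the overlapping actor, hides it, spawns an explosion effect and sound, and calls SayHiEvent on the first-person character.
; A timeline then blends the HUD's time and hammer-count backgrounds between translucent black and red.
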(event `self.Box.OnComponentBeginOverlap`
  (params (OverlappedComponent :type "PrimitiveComponent Object Reference") (OtherActor :type "Actor Object Reference") (OtherComp :type "PrimitiveComponent Object Reference") (OtherBodyIndex :type Integer) (bFromSweep :type Boolean) (SweepResult :type "HitResult Structure (by ref)"))
  (bind _miinterfaz (`/Game/FirstPerson/Blueprints/BP_FirstPersonCharacter.MiInterfaz` (cast `/Game/FirstPerson/Blueprints/BP_FirstPersonCharacter` (`GameplayStatics.GetPlayerCharacter` 0) :!pure true)))
  (bind _miinterfaz_2 (`/Game/FirstPerson/Blueprints/BP_FirstPersonCharacter.MiInterfaz` (cast `/Game/FirstPerson/Blueprints/BP_FirstPersonCharacter` (`GameplayStatics.GetPlayerCharacter` 0) :!pure true)))
  (`/Engine/EditorBlueprintResources/StandardMacros.DoOnce` false
    (:`Completed`
      (set `/Game/HunterGame_Levels/MyAssets/Blueprints/HUD/PlayerInterface.TiempoRestante` (+ (`/Game/HunterGame_Levels/MyAssets/Blueprints/HUD/PlayerInterface.TiempoRestante` _miinterfaz_2) 10.0) _miinterfaz_2)
      (`self.SetActorHiddenInGame` true)
      (`GameplayStatics.SpawnEmitterAtLocation` "/Game/InfinityBladeEffects/Effects/FX_Cines/cinema03/P_CIN_IB_Explosion.P_CIN_IB_Explosion" (`self.K2_GetActorLocation`) (struct) (0.5 0.5 0.5))
      (`GameplayStatics.PlaySoundAtLocation` "/Game/StarterContent/Audio/Explosion01.Explosion01" (0.0 0.0 0.0) (struct) 1.0 1.0 0.0 null null null null)
      (`/Game/FirstPerson/Blueprints/BP_FirstPersonCharacter.Say Hi Event` (cast `/Game/FirstPerson/Blueprints/BP_FirstPersonCharacter` (`GameplayStatics.GetPlayerCharacter` 0) :!pure true))
      (bind (_direction _newtrack_0) (`Timeline|Timeline_0` :!via `PlayFromStart`)
        (:`Update`
          (bind _returnvalue (`KismetMathLibrary.LinearColorLerp` (struct :`A` 0.3) (struct :`R` 0.633333 :`A` 1.0) _newtrack_0))
          (`Border.SetBrushColor` (`/Game/HunterGame_Levels/MyAssets/Blueprints/HUD/PlayerInterface.CuadradoDeTiempo` _miinterfaz) _returnvalue)
          (`Border.SetBrushColor` (`/Game/HunterGame_Levels/MyAssets/Blueprints/HUD/PlayerInterface.NumMartillosFondo` _miinterfaz) _returnvalue))))))

(fn `UserConstructionScript`)